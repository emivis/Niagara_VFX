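; BP_BakeTexture is an editor utility Blueprint that bakes a material into a static texture asset.
; BakeTexture checks that the render target and source material are valid, then draws the material into the render target.
; It then saves the result as a Texture2D named TextureFromRenderTarget through the editor-only render target conversion, so the bake does not work in packaged builds.
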(fn `BakeTexture`
  (if (and (`KismetSystemLibrary.IsValid` (`self.render target to draw`)) (`KismetSystemLibrary.IsValid` (`self.Material to draw from`)))
    (`KismetRenderingLibrary.DrawMaterialToRenderTarget` (`self.render target to draw`) (`self.Material to draw from`))
    (`KismetRenderingLibrary.RenderTargetCreateStaticTexture2DEditorOnly` (`self.render target to draw`) "TextureFromRenderTarget")))

(fn `UserConstructionScript`)